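; BP_GameOverZone is a trigger zone that ends play when certain NPCs overlap it.
; A runaway or stay NPC entering brings up the WB_GameOver widget, while a target NPC brings up WB_TargetEscaped.
; Both outcomes show the mouse cursor and switch the player controller to UI-only input focused on the new widget.
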(event `self.ReceiveActorBeginOverlap`
  (params (OtherActor :type "Actor Object Reference"))
  (bind _returnvalue (`GameplayStatics.GetPlayerController` 0))
  (bind _returnvalue_2 (`GameplayStatics.GetPlayerController` 0))
  (`|ExecutionSequence`
    (:`then_0`
      (cast `/Game/SHJ/BP/BP_RUNAWAYNPC` OtherActor
        (:`then`
          _)
        (:`CastFailed`
          (cast `/Game/SHJ/BP/BP_STAYNPC` OtherActor)))
      (bind _returnvalue_3 (`|CreateWidget` "/Game/SHJ/UI/WB_GameOver.WB_GameOver_C"))
      (`UserWidget.AddToViewport` _returnvalue_3 0)
      (set `PlayerController.bShowMouseCursor` true _returnvalue)
      (`WidgetBlueprintLibrary.SetInputMode_UIOnlyEx` _returnvalue _returnvalue_3))
    (:`then_1`
      (cast `/Game/SHJ/BP/BP_TARGETNPC` OtherActor)
      (bind _returnvalue_4 (`|CreateWidget` "/Game/SHJ/UI/WB_TargetEscaped.WB_TargetEscaped_C"))
      (`UserWidget.AddToViewport` _returnvalue_4 0)
      (set `PlayerController.bShowMouseCursor` true _returnvalue_2)
      (`WidgetBlueprintLibrary.SetInputMode_UIOnlyEx` _returnvalue_2 _returnvalue_4))))

(fn `UserConstructionScript`)