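; BP_MissionTrigger is a one-shot interaction actor that gives the player a new mission.
; It enables input for the first player controller on BeginPlay and tracks whether a BP_Player is inside its Trigger component through overlap events.
; Pressing F while in range passes NewMissionToSet to that player's UpdateMission through a DoOnce gate, then destroys the trigger.
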(event `self.ReceiveBeginPlay`
  (`self.EnableInput` (`GameplayStatics.GetPlayerController` 0)))

(event `self.Trigger.OnComponentBeginOverlap`
  (params (OverlappedComponent :type "PrimitiveComponent Object Reference") (OtherActor :type "Actor Object Reference") (OtherComp :type "PrimitiveComponent Object Reference") (OtherBodyIndex :type Integer) (bFromSweep :type Boolean) (SweepResult :type "HitResult Structure (by ref)"))
  (bind _asbp_player (cast `/Game/LC/Blueprint/BP_Player` OtherActor))
  (set `self.Is Within Range` true))

(event `Key|F` :consume false
  (params (Key :type "Key Structure"))
  (:`Pressed`
    (if (`self.Is Within Range`)
      (`/Engine/EditorBlueprintResources/StandardMacros.DoOnce` false
        (:`Completed`
          (`/Game/LC/Blueprint/BP_Player.UpdateMission` (stale `self.Trigger.OnComponentBeginOverlap` _asbp_player) (`self.NewMissionToSet`))
          (`self.K2_DestroyActor`))))))

(event `self.Trigger.OnComponentEndOverlap`
  (params (OverlappedComponent :type "PrimitiveComponent Object Reference") (OtherActor :type "Actor Object Reference") (OtherComp :type "PrimitiveComponent Object Reference") (OtherBodyIndex :type Integer))
  (cast `/Game/LC/Blueprint/BP_Player` OtherActor)
  (set `self.Is Within Range` false))

(fn `UserConstructionScript`)