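; Child door Blueprint that the player toggles with Interact and that certain NPCs open automatically.
; The Box trigger enables input and shows the Widget while the player overlaps it, and reverses both on exit.
; Interact alternates DoorOpen and DoorClose through a FlipFlop, which NPC-driven changes do not update.
; Overlapping BP_RUNAWAYNPC or BP_STAYNPC actors open the door on entry and close it on exit, only while IsSeeing is true.
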(event `EnhancedInput|/Game/SHJ/Inputs/Interact`
  (params (ActionValue :type Boolean) (ElapsedSeconds :type "Float (double-precision)") (TriggeredSeconds :type "Float (double-precision)") (InputAction :type "InputAction Object Reference" :default "/Game/SHJ/Inputs/Interact.Interact"))
  (:`Started`
    (`/Engine/EditorBlueprintResources/StandardMacros.FlipFlop`
      (:`A`
        (`self.Door_open`))
      (:`B`
        (`self.Door_close`)))))

(event `self.Box.OnComponentBeginOverlap`
  (params (OverlappedComponent :type "PrimitiveComponent Object Reference") (OtherActor :type "Actor Object Reference") (OtherComp :type "PrimitiveComponent Object Reference") (OtherBodyIndex :type Integer) (bFromSweep :type Boolean) (SweepResult :type "HitResult Structure (by ref)"))
  (if (== OtherActor (`GameplayStatics.GetPlayerCharacter` 0))
    (`self.EnableInput` (`GameplayStatics.GetPlayerController` 0))
    (`SceneComponent.SetHiddenInGame` (`self.Widget`) false false)
    (else
      (bind _asbp_runawaynpc (cast `/Game/SHJ/BP/BP_RUNAWAYNPC` OtherActor)
        (:`then`
          (if (`/Game/SHJ/BP/BP_RUNAWAYNPC.IsSeeing` _asbp_runawaynpc)
            (`self.Door_open`)))
        (:`CastFailed`
          (bind _asbp_staynpc (cast `/Game/SHJ/BP/BP_STAYNPC` OtherActor))
          (if (`/Game/SHJ/BP/BP_STAYNPC.IsSeeing` _asbp_staynpc)
            (`self.Door_open`)))))))

(event `self.Box.OnComponentEndOverlap`
  (params (OverlappedComponent :type "PrimitiveComponent Object Reference") (OtherActor :type "Actor Object Reference") (OtherComp :type "PrimitiveComponent Object Reference") (OtherBodyIndex :type Integer))
  (if (== OtherActor (`GameplayStatics.GetPlayerCharacter` 0))
    (`self.DisableInput` (`GameplayStatics.GetPlayerController` 0))
    (`SceneComponent.SetHiddenInGame` (`self.Widget`) true false)
    (else
      (bind _asbp_runawaynpc (cast `/Game/SHJ/BP/BP_RUNAWAYNPC` OtherActor)
        (:`then`
          (if (`/Game/SHJ/BP/BP_RUNAWAYNPC.IsSeeing` _asbp_runawaynpc)
            (`self.Door_close`)))
        (:`CastFailed`
          (bind _asbp_staynpc (cast `/Game/SHJ/BP/BP_STAYNPC` OtherActor))
          (if (`/Game/SHJ/BP/BP_STAYNPC.IsSeeing` _asbp_staynpc)
            (`self.Door_close`)))))))

(fn `UserConstructionScript`
  (`parent.UserConstructionScript`))