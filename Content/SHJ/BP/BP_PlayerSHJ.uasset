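; Player character for a stealth action game, with sprint, slide, crouch, jump, camera zoom, sword attacks, blink teleport and assassinations.
; Enhanced Input drives movement and abilities; blink places an indicator by camera trace, then teleports on release with an FOV and vignette timeline.
; A timer-driven camera sphere trace tracks interactables for the F key, which also moves nearby NPCs into paired takedown montages.
; It creates the HUD and mission widget, appending clues through UpdateMission.
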(event `Key|F`
  (params (Key :type "Key Structure"))
  (:`Pressed`
    (message `/Game/SHJ/BP/BP_Interaction.Interact` (`self.TraceItem`))))

(event `Create Interaction Trace`
  (`self.Interaction Trace`))

(event `self.ReceiveBeginPlay`
  ; Initialize
  (`|ExecutionSequence`
    (:`then_0`
      (`self.MappingContext`)
      ;[0 0.004652 0.15 0.5] (베타 추가) Clue
      (bind _returnvalue (`|CreateWidget` "/Game/SHJ/UI/WB_Mission.WB_Mission_C" (`GameplayStatics.GetPlayerController` 0)))
      (bind _output_get (set `self.Mission Widget` _returnvalue))
      (`UserWidget.AddToViewport` _output_get 0)
      (bind _returnvalue_2 (`KismetSystemLibrary.K2_SetTimer` null "Create Interaction Trace" 0.01))
      (set `self.Interaction Timer` _returnvalue_2)
      (bind _returnvalue_3 (`|CreateWidget` "/Game/SHJ/UI/UI_HUD.UI_HUD_C"))
      (`UserWidget.AddToViewport` _returnvalue_3 0))
    (:`then_1`
      (set `self.AttackDelay` 2.0)
      (set `self.BlinkDelay` 2.0))
    (:`then_2`
      (bind _returnvalue_4 (`|SpawnActorFromClass` "/Game/LC/Blueprint/BP_Sword.BP_Sword_C" (`self.GetTransform`) "Undefined" "MultiplyWithRoot" null null))
      (bind _output_get_2 (set `self.sword` _returnvalue_4))
      (`/Engine/EditorBlueprintResources/StandardMacros.IsValid` _output_get_2
        (:`Is Valid`
          (`self.K2_AttachToComponent` (`self.sword`) (`self.Mesh`) "sword_socket" "SnapToTarget" "SnapToTarget" "KeepRelative" true))))))

(event `self.ReceiveTick`
  (params (DeltaSeconds :type "Float (single-precision)"))
  (bind _output_get (set `self.Delta Seconds` DeltaSeconds))
  (`|ExecutionSequence`
    (:`then_0`
      ; attack
      (bind _output_get_2 (set `self.AttackDelay` (+ _output_get (`self.AttackDelay`)))))
    (:`then_1`
      (bind _output_get_3 (set `self.BlinkDelay` (+ _output_get (`self.BlinkDelay`)))))))

(event `EnhancedInput|/Game/LC/Input/IA_Crouch`
  (params (ActionValue :type Boolean) (ElapsedSeconds :type "Float (double-precision)") (TriggeredSeconds :type "Float (double-precision)") (InputAction :type "InputAction Object Reference" :default "/Game/LC/Input/IA_Crouch.IA_Crouch"))
  (bind _charactermovement (`self.CharacterMovement`))
  (bind _charactermovement_2 (`self.CharacterMovement`))
  (bind (_returnvalue_x _returnvalue_y) (`KismetMathLibrary.BreakVector` (* (`KismetMathLibrary.Normal` (`self.GetActorForwardVector`)) 2000)))
  ; crouch toggle & sliding
  (:`Started`
    (if (`self.isSprinting`)
      (if (not (`self.isSliding`))
        (`self.Crouch`)
        (set `self.isSliding` true)
        (`self.LaunchCharacter` (`KismetMathLibrary.MakeVector` _returnvalue_x _returnvalue_y) true)
        (set `CharacterMovementComponent.BrakingFrictionFactor` 0.0 _charactermovement)
        (set `CharacterMovementComponent.GroundFriction` 4.0 _charactermovement)
        (`KismetSystemLibrary.Delay` 1.0)
        (set `self.isSliding` false)
        (set `CharacterMovementComponent.BrakingFrictionFactor` 2.0 _charactermovement_2)
        (set `CharacterMovementComponent.GroundFriction` 8.0 _charactermovement_2))
      (else
        ;; simple crouch and uncrouch
        (`/Engine/EditorBlueprintResources/StandardMacros.FlipFlop`
          (:`A`
            (`self.Crouch`))
          (:`B`
            (`self.UnCrouch`)))))))

(event `EnhancedInput|/Game/LC/Input/IA_Attack`
  (params (ActionValue :type Boolean) (ElapsedSeconds :type "Float (double-precision)") (TriggeredSeconds :type "Float (double-precision)") (InputAction :type "InputAction Object Reference" :default "/Game/LC/Input/IA_Attack.IA_Attack"))
  (bind _mesh (`self.Mesh`))
  ; attack
  (:`Started`
    (if (>= (stale `self.ReceiveTick` _output_get_2) 2.0)
      (set `self.AttackDelay` 0.0)
      (`/Engine/EditorBlueprintResources/StandardMacros.FlipFlop`
        (:`A`
          (`|PlayMontage` _mesh "/Game/LC/Characters/Player/Anim/Attack/AM_InwardSlash_Montage.AM_InwardSlash_Montage" 1.0 0.0 "None" false))
        (:`B`
          (`|PlayMontage` _mesh "/Game/LC/Characters/Player/Anim/Attack/AM_OutwardSlash_Montage.AM_OutwardSlash_Montage" 1.0 0.0 "None" false))))))

(event `EnhancedInput|/Game/LC/Input/IA_Ability`
  (params (ActionValue :type Boolean) (ElapsedSeconds :type "Float (double-precision)") (TriggeredSeconds :type "Float (double-precision)") (InputAction :type "InputAction Object Reference" :default "/Game/LC/Input/IA_Ability.IA_Ability"))
  (bind _camera (`self.Camera`))
  (bind _indicator (`self.Indicator`))
  (bind _indicator_2 (`self.Indicator`))
  (bind _returnvalue (`self.K2_GetActorLocation` _indicator_2))
  ; blink
  (:`Triggered`
    (`/Engine/EditorBlueprintResources/StandardMacros.IsValid` _indicator :!label _label
      (:`Is Valid`
        (bind _returnvalue_2 (>= (stale `self.ReceiveTick` _output_get_3) 0.4))
        (if _returnvalue_2
          (bind (_returnvalue_3 _returnvalue2) (`self.RayCalc`))
          (bind _outhit (`KismetSystemLibrary.LineTraceSingle` :`Start` _returnvalue_3 :`End` _returnvalue2 :`TraceChannel` "TraceTypeQuery1" :`DrawDebugType` "ForDuration"))
          (bind (_bblockinghit _binitialoverlap _time _distance _location _impactpoint _normal _impactnormal _physmat _hitactor _hitcomponent _hitbonename _bonename _hititem _elementindex _faceindex _tracestart _traceend) (`GameplayStatics.BreakHitResult` _outhit))
          (if _bblockinghit
            (`self.K2_SetActorLocation` _indicator _location false false)
            (else
              (`self.K2_SetActorLocation` _indicator _traceend false false)))))
      (:`Is Not Valid`
        (if _returnvalue_2
          (bind (_returnvalue_4 _returnvalue2_2) (`self.RayCalc`))
          (bind _outhit_2 (`KismetSystemLibrary.LineTraceSingle` :`Start` _returnvalue_4 :`End` _returnvalue2_2 :`TraceChannel` "TraceTypeQuery1" :`DrawDebugType` "ForDuration"))
          (bind (_bblockinghit_2 _binitialoverlap_2 _time_2 _distance_2 _location_2 _impactpoint_2 _normal_2 _impactnormal_2 _physmat_2 _hitactor_2 _hitcomponent_2 _hitbonename_2 _bonename_2 _hititem_2 _elementindex_2 _faceindex_2 _tracestart_2 _traceend_2) (`GameplayStatics.BreakHitResult` _outhit_2))
          (if _bblockinghit_2
            (bind _returnvalue_5 (`|SpawnActorFromClass` "/Game/LC/Blueprint/BP_BlinkIndicator.BP_BlinkIndicator_C" (`KismetMathLibrary.MakeTransform` _location_2) "Undefined" "MultiplyWithRoot" null null))
            (set `self.Indicator` _returnvalue_5)
            (else
              (bind _returnvalue_6 (`|SpawnActorFromClass` "/Game/LC/Blueprint/BP_BlinkIndicator.BP_BlinkIndicator_C" (`KismetMathLibrary.MakeTransform` _traceend_2) "Undefined" "MultiplyWithRoot" null null))
              (set `self.Indicator` _returnvalue_6)))))))
  (:`Started`
    (goto _label))
  (:`Completed`
    (`/Engine/EditorBlueprintResources/StandardMacros.IsValid` _indicator_2
      (:`Is Valid`
        (if _returnvalue_2
          (`self.K2_SetActorLocation` (- _returnvalue (* (`KismetMathLibrary.Normal` (- (`self.K2_GetActorLocation`) _returnvalue)) 1e-05)))
          (`self.K2_DestroyActor` _indicator_2)
          (bind (_direction _newtrack_0) (`Timeline|blinkeffect` :!via `PlayFromStart`)
            (:`Update`
              (`CameraComponent.SetFieldOfView` _camera _newtrack_0)
              (set `CameraComponent.PostProcessSettings` (make `PostProcessSettings` :`VignetteIntensity` (`KismetMathLibrary.MapRangeClamped` _newtrack_0 90.0 150.0 0.0 1.0)) _camera)
              (set `self.BlinkDelay` 0.0))))))))

(event `EnhancedInput|/Game/LC/Input/IA_Zoom`
  (params (ActionValue :type Boolean) (ElapsedSeconds :type "Float (double-precision)") (TriggeredSeconds :type "Float (double-precision)") (InputAction :type "InputAction Object Reference" :default "/Game/LC/Input/IA_Zoom.IA_Zoom"))
  (bind _camera (`self.Camera`))
  ; camera zoom in
  (:`Started`
    (`/Engine/EditorBlueprintResources/StandardMacros.FlipFlop`
      (:`A`
        (bind (_direction _newtrack_0) (`Timeline|90-60` :!label _label_2)
          (:`Update`
            (`CameraComponent.SetFieldOfView` _camera _newtrack_0)
            (set `CameraComponent.PostProcessSettings` (make `PostProcessSettings` :`VignetteIntensity` (`KismetMathLibrary.MapRangeClamped` _newtrack_0 90.0 60.0 0.0 1.0)) _camera))))
      (:`B`
        (goto _label_2 :!via `Reverse`)))))

(event `Key|F`
  (params (Key :type "Key Structure"))
  (bind (_returnvalue_location _returnvalue_rotation) (`KismetMathLibrary.BreakTransform` (`SceneComponent.K2_GetComponentToWorld` (`self.REF Pose`))))
  ; Assassination(Runaway)
  (:`Pressed`
    (bind (_outactors _returnvalue) (`KismetSystemLibrary.SphereOverlapActors` (`self.K2_GetActorLocation`) 200.0 (`|MakeArray` "ObjectTypeQuery3" :!type "EObjectTypeQuery Enum")))
    (if _returnvalue
      (for _array_element _outactors
        (if (`self.ActorHasTag` _array_element "NPC")
          (bind _asbp_runawaynpc (cast `/Game/SHJ/BP/BP_RUNAWAYNPC` _array_element))
          (if (not (`/Game/SHJ/BP/BP_RUNAWAYNPC.IsDead` _asbp_runawaynpc))
            (`/Game/SHJ/BP/BP_RUNAWAYNPC.Move To` _asbp_runawaynpc _returnvalue_location _returnvalue_rotation)
            (set `/Game/SHJ/BP/BP_RUNAWAYNPC.IsDead` true _asbp_runawaynpc)
            (`self.DisableInput` null)
            (`self.PlayAnimMontage` "/Game/SHJ/Animation/Paired_Knife_Stealth_KidneyAndNeck_Att_Montage.Paired_Knife_Stealth_KidneyAndNeck_Att_Montage")
            (`KismetSystemLibrary.Delay` 2.0)
            (`self.EnableInput` null)))))))

(event `Key|F`
  (params (Key :type "Key Structure"))
  (bind (_returnvalue_location _returnvalue_rotation) (`KismetMathLibrary.BreakTransform` (`SceneComponent.K2_GetComponentToWorld` (`self.REF Pose`))))
  ;[0.006758 0.001016 0.15 0.5] Assassination(Stay)
  (:`Pressed`
    (bind (_outactors _returnvalue) (`KismetSystemLibrary.SphereOverlapActors` (`self.K2_GetActorLocation`) 200.0 (`|MakeArray` "ObjectTypeQuery3" :!type "EObjectTypeQuery Enum")))
    (if _returnvalue
      (for _array_element _outactors
        (if (`self.ActorHasTag` _array_element "NPC")
          (bind _asbp_staynpc (cast `/Game/SHJ/BP/BP_STAYNPC` _array_element))
          (if (not (`/Game/SHJ/BP/BP_STAYNPC.IsDead` _asbp_staynpc))
            (`/Game/SHJ/BP/BP_STAYNPC.Move To` _asbp_staynpc _returnvalue_location _returnvalue_rotation)
            (set `/Game/SHJ/BP/BP_STAYNPC.IsDead` true _asbp_staynpc)
            (`self.DisableInput` null)
            (`self.PlayAnimMontage` "/Game/SHJ/Animation/Paired_Knife_Stealth_KidneyAndNeck_Att_Montage.Paired_Knife_Stealth_KidneyAndNeck_Att_Montage")
            (`KismetSystemLibrary.Delay` 2.0)
            (`self.EnableInput` null)))))))

(event `Key|F`
  (params (Key :type "Key Structure"))
  (bind (_returnvalue_location _returnvalue_rotation) (`KismetMathLibrary.BreakTransform` (`SceneComponent.K2_GetComponentToWorld` (`self.REF Pose`))))
  ;[0.00145 0 0.15 0.5] Assassination(Target)
  (:`Pressed`
    (bind (_outactors _returnvalue) (`KismetSystemLibrary.SphereOverlapActors` (`self.K2_GetActorLocation`) 200.0 (`|MakeArray` "ObjectTypeQuery3" :!type "EObjectTypeQuery Enum")))
    (if _returnvalue
      (for _array_element _outactors
        (if (`self.ActorHasTag` _array_element "NPC")
          (bind _asbp_targetnpc (cast `/Game/SHJ/BP/BP_TARGETNPC` _array_element))
          (if (not (`/Game/SHJ/BP/BP_TARGETNPC.IsDead` _asbp_targetnpc))
            (`/Game/SHJ/BP/BP_TARGETNPC.Move To` _asbp_targetnpc _returnvalue_location _returnvalue_rotation)
            (set `/Game/SHJ/BP/BP_TARGETNPC.IsDead` false _asbp_targetnpc)
            (`self.DisableInput` null)
            (`self.PlayAnimMontage` "/Game/SHJ/Animation/Paired_Knife_Stealth_KidneyAndNeck_Att_Montage.Paired_Knife_Stealth_KidneyAndNeck_Att_Montage")
            (`KismetSystemLibrary.Delay` 2.0)
            (`self.EnableInput` null)))))))

(event `EnhancedInput|/Game/LC/Input/IA_Sprint`
  (params (ActionValue :type Boolean) (ElapsedSeconds :type "Float (double-precision)") (TriggeredSeconds :type "Float (double-precision)") (InputAction :type "InputAction Object Reference" :default "/Game/LC/Input/IA_Sprint.IA_Sprint"))
  (bind _charactermovement (`self.CharacterMovement`))
  ; sprint
  (:`Triggered`
    (if (and (`NavMovementComponent.IsMovingOnGround` _charactermovement) (not (`self.isSliding`)))
      (if (`NavMovementComponent.IsCrouching` _charactermovement)
        (`self.UnCrouch`))
      (set `CharacterMovementComponent.MaxWalkSpeed` 900.0 _charactermovement)
      (set `self.isSprinting` true)))
  (:`Completed`
    (set `CharacterMovementComponent.MaxWalkSpeed` 600.0 _charactermovement)
    (set `self.isSprinting` false)))

(event `EnhancedInput|/Game/LC/Input/IA_Look`
  (params (ActionValue :type "Vector2D Structure") (ElapsedSeconds :type "Float (double-precision)") (TriggeredSeconds :type "Float (double-precision)") (InputAction :type "InputAction Object Reference" :default "/Game/LC/Input/IA_Look.IA_Look"))
  ; camera rotation
  (:`Triggered`
    (`self.AddControllerYawInput` ActionValue_X)
    (`self.AddControllerPitchInput` ActionValue_Y)))

(event `EnhancedInput|/Game/LC/Input/IA_Jump`
  (params (ActionValue :type Boolean) (ElapsedSeconds :type "Float (double-precision)") (TriggeredSeconds :type "Float (double-precision)") (InputAction :type "InputAction Object Reference" :default "/Game/LC/Input/IA_Jump.IA_Jump"))
  ; basic move
  ;; jump + double jump
  (:`Started`
    (`self.UnCrouch`)
    (`self.Jump`)))

(event `EnhancedInput|/Game/LC/Input/IA_WS`
  (params (ActionValue :type "Float (double-precision)") (ElapsedSeconds :type "Float (double-precision)") (TriggeredSeconds :type "Float (double-precision)") (InputAction :type "InputAction Object Reference" :default "/Game/LC/Input/IA_WS.IA_WS"))
  (bind (_returnvalue_roll _returnvalue_pitch _returnvalue_yaw) (`KismetMathLibrary.BreakRotator` (`self.GetControlRotation`)))
  ; basic move
  ;; movement
  ;;; ws movement
  (:`Triggered`
    (`self.AddMovementInput` (`KismetMathLibrary.GetForwardVector` (`KismetMathLibrary.MakeRotator` 0.0 0.0 _returnvalue_yaw)) ActionValue)))

(event `EnhancedInput|/Game/LC/Input/IA_AD`
  (params (ActionValue :type "Float (double-precision)") (ElapsedSeconds :type "Float (double-precision)") (TriggeredSeconds :type "Float (double-precision)") (InputAction :type "InputAction Object Reference" :default "/Game/LC/Input/IA_AD.IA_AD"))
  (bind (_returnvalue_roll _returnvalue_pitch _returnvalue_yaw) (`KismetMathLibrary.BreakRotator` (`self.GetControlRotation`)))
  ; basic move
  ;; movement
  ;;; ad movement
  (:`Triggered`
    (`self.AddMovementInput` (`KismetMathLibrary.GetRightVector` (`KismetMathLibrary.MakeRotator` _returnvalue_roll 0.0 _returnvalue_yaw)) ActionValue)))

(fn `Interaction Trace`
  (bind _camera (`self.Camera`))
  (bind _traceitem (`self.TraceItem`))
  (bind _returnvalue (`SceneComponent.K2_GetComponentLocation` _camera))
  (bind _outhit (`KismetSystemLibrary.SphereTraceSingle` _returnvalue (+ _returnvalue (* (`KismetMathLibrary.GetForwardVector` (`SceneComponent.K2_GetComponentRotation` _camera)) 1000)) 0.0 "TraceTypeQuery1"))
  (bind (_bblockinghit _binitialoverlap _time _distance _location _impactpoint _normal _impactnormal _physmat _hitactor) (`GameplayStatics.BreakHitResult` _outhit))
  (if (`KismetSystemLibrary.DoesImplementInterface` _hitactor)
    (if (!= _hitactor _traceitem)
      (bind _output_get (set `self.TraceItem` _hitactor))
      (message `/Game/SHJ/BP/BP_Interaction.Can Receive Trace` _output_get true))
    (else
      (message `/Game/SHJ/BP/BP_Interaction.Can Receive Trace` _traceitem false)
      (set `self.TraceItem` null))))

(fn `MappingContext`
  (bind _returnvalue (`GameplayStatics.GetPlayerController` 0))
  (`EnhancedInputSubsystemInterface.AddMappingContext` (pcsubsystem `EnhancedInputLocalPlayerSubsystem` (`GameplayStatics.GetPlayerController` 0)) "/Game/LC/Input/IMC_Player.IMC_Player" 0 (struct))
  (set `PlayerController.bShowMouseCursor` false _returnvalue)
  (`WidgetBlueprintLibrary.SetInputMode_GameOnly` _returnvalue))

(fn `MoveFunction`
  (params (A :type "Float (single-precision)"))
  (`self.K2_SetActorLocation` (+ (* (`self.movement_speed`) (`KismetMathLibrary.Normal` (+ (* (`|GetInputActionValue`) (0.0 0.0 0.0)) (* (`|GetInputActionValue`) (`self.GetActorForwardVector`)))) A) (`self.K2_GetActorLocation`))))

(fn `RayCalc`
  (returns (ReturnValue :type "Vector Structure") (ReturnValue2 :type "Vector Structure"))
  (bind _camera (`self.Camera`))
  (bind _returnvalue (`SceneComponent.K2_GetComponentLocation` _camera))
  (return _returnvalue (+ _returnvalue (* (`SceneComponent.GetForwardVector` _camera) 1000.0))))

(fn `UpdateMission`
  (params (currentMission :type String))
  (bind _returnvalue (`|CreateWidget` "/Game/SHJ/UI/WB_ClueItem.WB_ClueItem_C"))
  (`TextBlock.SetText` (`/Game/SHJ/UI/WB_ClueItem.ClueText` _returnvalue) (`KismetTextLibrary.Conv_StringToText` currentMission))
  (`VerticalBox.AddChildToVerticalBox` (`/Game/SHJ/UI/WB_Mission.ClueList` (`self.Mission Widget`)) _returnvalue))

(fn `UserConstructionScript`)