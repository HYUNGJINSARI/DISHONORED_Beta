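; BP_RUNAWAYNPC is an innocent NPC that patrols and flees from the player.
; It loops through four tagged actors, sprints away when AIPerception detects the player, and resumes patrol when the player is forgotten.
; RunAway repeatedly projects a distant point opposite the player onto the navmesh and randomizes it.
; MoveTo plays the stealth-kill victim montage, disables movement and shows the innocent-kill widget after a delay.
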(event `self.ReceiveBeginPlay`
  (add `AIPerceptionComponent.OnTargetPerceptionForgotten` (`self.AIPerception`) (delegate `OnTargetPerceptionForgotten_Event`))
  (bind _outactors (`GameplayStatics.GetAllActorsWithTag` (`self.Tag`) :!label _label))
  (`|AIMoveTo` self (0.0 0.0 0.0) (`|GetArrayItem` _outactors (`self.CurrentIndex`))
    (:`OnSuccess`
      ; 4지점 반복순회
      (set `self.CurrentIndex` (mod (+ (`self.CurrentIndex`) 1) 4))
      (`KismetSystemLibrary.Delay` 1.0)
      (goto _label))))

(event `OnTargetPerceptionForgotten_Event`
  (params (Actor :type "Actor Object Reference"))
  (`KismetSystemLibrary.PrintString` (`KismetTextLibrary.Conv_TextToString` (`|FormatText` "AL Forget this {actor}" Actor))))

(event `self.AIPerception.OnTargetPerceptionForgotten`
  (params (Actor :type "Actor Object Reference"))
  (cast `/Game/LC/Blueprint/BP_Player` Actor)
  (set `CharacterMovementComponent.MaxWalkSpeed` 300.0 (`self.CharacterMovement`))
  (goto _label))

(event `self.AIPerception.OnTargetPerceptionUpdated`
  (params (Actor :type "Actor Object Reference") (Stimulus :type "AIStimulus Structure"))
  (if (== Actor (`GameplayStatics.GetPlayerCharacter` 0))
    (cast `/Game/LC/Blueprint/BP_Player` Actor)
    (set `CharacterMovementComponent.MaxWalkSpeed` 500.0 (`self.CharacterMovement`))
    (set `self.Char REF` Actor)
    (set `self.IsSeeing` true)
    (`self.RunAway`)))

(event `RunAway`
  (bind _returnvalue (`self.K2_GetActorLocation`))
  (`|AIMoveTo` self (`NavigationSystemV1.K2_GetRandomReachablePointInRadius` (`NavigationSystemV1.K2_ProjectPointToNavigation` (`KismetMathLibrary.MakeVector` (.x (+ _returnvalue (* (`KismetMathLibrary.GetForwardVector` (`KismetMathLibrary.FindLookAtRotation` _returnvalue (`self.K2_GetActorLocation` (`self.Char REF`)))) -10000.0))) (.y (+ _returnvalue (* (`KismetMathLibrary.GetForwardVector` (`KismetMathLibrary.FindLookAtRotation` _returnvalue (`self.K2_GetActorLocation` (`self.Char REF`)))) -10000.0))) (.z _returnvalue)) null null (10000.0 10000.0 10000.0)) 0.0 null null) null
    (:`OnSuccess`
      _)
    (:`OnFail`
      _))
  (`self.RunAway`))

(event `self.ReceiveTick`
  (params (DeltaSeconds :type "Float (single-precision)"))
  ; 디버그
  (`KismetSystemLibrary.DrawDebugConeInDegrees` (`self.K2_GetActorLocation`) (* (`self.GetActorForwardVector`) -10000.0) -400.0 30.0 30.0 12 (struct :`R` 1.0 :`A` 1.0)))

(event `Move To`
  (params (Location :type "Vector Structure") (Rotation :type "Rotator Structure"))
  (bind _returnvalue (`GameplayStatics.GetPlayerController` 0))
  (`/Engine/EditorBlueprintResources/StandardMacros.DoOnce` (`self.IsDead`)
    (:`Completed`
      (`|ExecutionSequence`
        (:`then_0`
          (`|AIMoveTo` self Location null))
        (:`then_1`
          (`self.PlayAnimMontage` "/Game/SHJ/Animation/Paired_Knife_Stealth_KidneyAndNeck_Vic_Montage.Paired_Knife_Stealth_KidneyAndNeck_Vic_Montage")
          (`self.K2_SetActorRotation` Rotation)
          (`MovementComponent.StopMovementImmediately` (`self.CharacterMovement`))
          (`PrimitiveComponent.SetCollisionEnabled` (`self.CapsuleComponent`) "QueryAndPhysics")
          (`CharacterMovementComponent.SetMovementMode` (`self.CharacterMovement`) "MOVE_None" 0)
          (set `self.bUseControllerRotationYaw` false)
          (`self.SetActorTickEnabled` false)
          (`ActorComponent.SetComponentTickEnabled` (`self.AIPerception`) false)
          ; 무고한 사람을 죽인 죄
          (`KismetSystemLibrary.Delay` 3.0)
          (bind _returnvalue_2 (`|CreateWidget` "/Game/SHJ/UI/WB_Kill_Innocent.WB_Kill_Innocent_C"))
          (`UserWidget.AddToViewport` _returnvalue_2 0)
          (set `PlayerController.bShowMouseCursor` true _returnvalue)
          (`WidgetBlueprintLibrary.SetInputMode_UIOnlyEx` _returnvalue _returnvalue_2))))))

(fn `UserConstructionScript`)