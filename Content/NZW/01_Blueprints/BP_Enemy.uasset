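; Enemy character that carries a pistol and sword, targets the player, and can be killed by a paired stealth takedown.
; BeginPlay gathers tagged patrol points and attaches both spawned weapons to sockets; helper functions re-attach them.
; Tick sets walk speed from combat, draw and attack flags, flags death at zero HP, and sphere-traces the blade during attacks, damaging the player once per swing.
; StealthDead moves the enemy into position before playing the victim montage.
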(event `self.ReceiveBeginPlay`
  (set `self.Combat State` "NewEnumerator4")
  (`|ExecutionSequence`
    (:`then_0`
      (set `self.HP` (`self.MaxHP`))
      (set `self.Target` (`GameplayStatics.GetPlayerPawn` 0)))
    (:`then_1`
      ; Tag로 이동경로 액터 모으기
      (bind _outactors (`GameplayStatics.GetAllActorsWithTag` (`self.PatrolLocationTag`)))
      (set `self.PatrolPoints` _outactors))
    (:`then_2`
      (bind _returnvalue (`|SpawnActorFromClass` "/Game/NZW/01_Blueprints/Weapons/BP_Enemy_Pistol.BP_Enemy_Pistol_C" (`self.GetTransform`) "Undefined" "MultiplyWithRoot" null null))
      (bind _output_get (set `self.Pistol` _returnvalue))
      (`/Engine/EditorBlueprintResources/StandardMacros.IsValid` _output_get
        (:`Is Valid`
          (`self.K2_AttachToComponent` (`self.Pistol`) (`self.Mesh`) (`self.PistolUnarmedSocket`) "SnapToTarget" "SnapToTarget" "KeepRelative" false))))
    (:`then_3`
      (bind _returnvalue_2 (`|SpawnActorFromClass` "/Game/NZW/01_Blueprints/Weapons/BP_Enemy_Sword.BP_Enemy_Sword_C" (`self.GetTransform`) "Undefined" "MultiplyWithRoot" null null))
      (bind _output_get_2 (set `self.Sword` _returnvalue_2))
      (`/Engine/EditorBlueprintResources/StandardMacros.IsValid` _output_get_2
        (:`Is Valid`
          (`self.K2_AttachToComponent` (`self.Sword`) (`self.Mesh`) (`self.SwordUnarmedSocket`) "SnapToTarget" "SnapToTarget" "KeepRelative" false))))))

(event `self.ReceiveTick`
  (params (DeltaSeconds :type "Float (single-precision)"))
  (bind _mesh (`self.Mesh`))
  (`|ExecutionSequence`
    (:`then_0`
      ; 플레이어 감지 시 Walk Speed 변경
      (if (`self.IsCombat`)
        (if (or (`self.IsPistolDrawEnd`) (`self.IsSwordDrawEnd`))
          (if (`self.IsAttack`)
            (set `CharacterMovementComponent.MaxWalkSpeed` 0.0 (`self.CharacterMovement`))
            (else
              (set `CharacterMovementComponent.MaxWalkSpeed` 450.0 (`self.CharacterMovement`))))
          (else
            (set `CharacterMovementComponent.MaxWalkSpeed` 0.0 (`self.CharacterMovement`))))
        (else
          (set `CharacterMovementComponent.MaxWalkSpeed` 300.0 (`self.CharacterMovement`)))))
    (:`then_1`
      (if (<= (`self.HP`) 0.0)
        (set `self.IsDead` true)))
    (:`then_2`
      (if (`self.IsAttacking`)
        (bind (_outhit _returnvalue) (`KismetSystemLibrary.SphereTraceSingleForObjects` (`SceneComponent.GetSocketLocation` _mesh "SwordBase") (`SceneComponent.GetSocketLocation` _mesh "SwordTip") 20.0 (`|MakeArray` "ObjectTypeQuery8" :!type "EObjectTypeQuery Enum")))
        (if _returnvalue
          (bind (_bblockinghit _binitialoverlap _time _distance _location _impactpoint _normal _impactnormal _physmat _hitactor) (`GameplayStatics.BreakHitResult` _outhit))
          (if (not (`KismetArrayLibrary.Array_Contains` (`self.HitActors`) _hitactor))
            (`KismetArrayLibrary.Array_Add` (`self.HitActors`) _hitactor)
            (bind _asbp_player (cast `/Game/LC/Blueprint/BP_Player` _hitactor))
            (`/Game/LC/Blueprint/BP_Player.GetHit` _asbp_player 25.0)))
        (else
          (`KismetArrayLibrary.Array_Clear` (`self.HitActors`)))))))

(event `self.CapsuleComponent.OnComponentHit`
  (params (HitComponent :type "PrimitiveComponent Object Reference") (OtherActor :type "Actor Object Reference") (OtherComp :type "PrimitiveComponent Object Reference") (NormalImpulse :type "Vector Structure") (Hit :type "HitResult Structure (by ref)"))
  (if (== OtherActor (`GameplayStatics.GetPlayerPawn` 0))
    (set `self.IsPlayerDetected` true)))

(event `StealthDead`
  (params (Destination :type "Vector Structure") (Rotation :type "Rotator Structure"))
  (set `self.IsStealthDead` true)
  (`|AIMoveTo` null Destination null
    (:`then`
      (`self.K2_SetActorRotation` Rotation)
      (`MovementComponent.StopMovementImmediately` (`self.CharacterMovement`))
      (`self.PlayEnemyMontage` "/Game/NZW/01_Blueprints/Animation/Montage/AMT_Paired_Stealth_vic.AMT_Paired_Stealth_vic"))))

(fn `AttatchPistol`
  (params (AttachName :type Name))
  (`self.K2_AttachToComponent` (`self.Pistol`) (`self.Mesh`) AttachName "SnapToTarget" "SnapToTarget" "KeepRelative" false))

(fn `AttatchSword`
  (params (AttachName :type Name))
  (`self.K2_AttachToComponent` (`self.Sword`) (`self.Mesh`) AttachName "SnapToTarget" "SnapToTarget" "KeepRelative" false))

(fn `DebugText`
  (params (TextLocation :type "Vector Structure" :default (0.0 0.0 100.0)) (Text :type String) (TextColor :type "LinearColor Structure")))

(fn `EnemyGetHit`
  (params (Damage :type "Float (double-precision)"))
  (set `self.HP` (- (`self.HP`) Damage)))

(fn `PlayEnemyMontage`
  (params (AnimMontage :type "AnimMontage Object Reference"))
  (if (not (`AnimInstance.Montage_IsPlaying` (`SkeletalMeshComponent.GetAnimInstance` (`self.Mesh`)) AnimMontage))
    (set `self.IsAttack` true)
    (`self.PlayAnimMontage` AnimMontage)))

(fn `RangeChecking`
  (params (Range :type "Float (double-precision)"))
  (returns (Result :type Boolean))
  (return (< (`KismetMathLibrary.Vector_Distance` (`self.K2_GetActorLocation` (`self.Target`)) (`self.K2_GetActorLocation`)) Range)))

(fn `UserConstructionScript`)