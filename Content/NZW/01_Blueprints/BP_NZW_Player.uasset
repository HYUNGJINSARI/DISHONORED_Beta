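; First-person or third-person player character with Enhanced Input movement, sprint, crouch, zoom, blink teleport and stealth kills.
; Holding the ability places an indicator by camera trace; release teleports there with an FOV/vignette effect and cooldown.
; F messages the timer-triggered camera trace's interactable and sphere-overlaps nearby living NPCs or enemies for a montage-driven assassination.
; Attack input only resets its cooldown; debug drawing remains in blink and assassination.
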(event `EnhancedInput|/Game/LC/Input/IA_Jump`
  (params (ActionValue :type Boolean) (ElapsedSeconds :type "Float (double-precision)") (TriggeredSeconds :type "Float (double-precision)") (InputAction :type "InputAction Object Reference" :default "/Game/LC/Input/IA_Jump.IA_Jump"))
  ; jump + double jump
  (:`Started`
    (`self.Jump`)))

(event `EnhancedInput|/Game/LC/Input/IA_Crouch`
  (params (ActionValue :type Boolean) (ElapsedSeconds :type "Float (double-precision)") (TriggeredSeconds :type "Float (double-precision)") (InputAction :type "InputAction Object Reference" :default "/Game/LC/Input/IA_Crouch.IA_Crouch"))
  ; crouch toggle
  (:`Started`
    (`/Engine/EditorBlueprintResources/StandardMacros.FlipFlop`
      (:`A`
        (`self.Crouch`))
      (:`B`
        (`self.UnCrouch`)))))

(event `Key|F`
  (params (Key :type "Key Structure"))
  ;[0.1356 0.07421 0.15 0.502] 인게임 인터렉션 관련 UI 출력 코드
  (:`Pressed`
    (message `/Game/SHJ/BP/BP_Interaction.Interact` (`self.Trace item`))))

(event `Create Interaction Trace`
  ;[0.1356 0.07421 0.15 0.502] 인게임 인터렉션 관련 UI 출력 코드
  (`self.Interaction Trace`))

(event `self.ReceiveBeginPlay`
  (`|ExecutionSequence`
    (:`then_0`
      (`self.MappingContext`)
      ;[0.1356 0.07421 0.15 0.502] 인게임 인터렉션 관련 UI 출력 코드
      (bind _returnvalue (`KismetSystemLibrary.K2_SetTimer` null "Create Interaction Trace" 0.01))
      (set `self.Interaction Timer` _returnvalue)
      (bind _returnvalue_2 (`|CreateWidget` "/Game/SHJ/UI/UI_HUD.UI_HUD_C"))
      (`UserWidget.AddToViewport` _returnvalue_2 0))
    (:`then_1`
      (set `self.AttackDelay` 2.0)
      (set `self.BlinkDelay` 2.0))))

(event `EnhancedInput|/Game/LC/Input/IA_Look`
  (params (ActionValue :type "Vector2D Structure") (ElapsedSeconds :type "Float (double-precision)") (TriggeredSeconds :type "Float (double-precision)") (InputAction :type "InputAction Object Reference" :default "/Game/LC/Input/IA_Look.IA_Look"))
  ; camera rotation
  (:`Triggered`
    (`self.AddControllerYawInput` ActionValue_X)
    (`self.AddControllerPitchInput` ActionValue_Y)))

(event `EnhancedInput|/Game/LC/Input/IA_Zoom`
  (params (ActionValue :type Boolean) (ElapsedSeconds :type "Float (double-precision)") (TriggeredSeconds :type "Float (double-precision)") (InputAction :type "InputAction Object Reference" :default "/Game/LC/Input/IA_Zoom.IA_Zoom"))
  (bind _camera (`self.Camera`))
  ; camera zoom in
  (:`Started`
    (`/Engine/EditorBlueprintResources/StandardMacros.FlipFlop`
      (:`A`
        (bind (_direction _newtrack_0) (`Timeline|90-60` :!label _label)
          (:`Update`
            (`CameraComponent.SetFieldOfView` _camera _newtrack_0)
            (set `CameraComponent.PostProcessSettings` (make `PostProcessSettings` :`VignetteIntensity` (`KismetMathLibrary.MapRangeClamped` _newtrack_0 90.0 60.0 0.0 1.0)) _camera))))
      (:`B`
        (goto _label :!via `Reverse`)))))

(event `self.ReceiveTick`
  (params (DeltaSeconds :type "Float (single-precision)"))
  (bind _output_get (set `self.Delta Seconds` DeltaSeconds))
  (`|ExecutionSequence`
    (:`then_0`
      ; attack
      (bind _output_get_2 (set `self.AttackDelay` (+ _output_get (`self.AttackDelay`)))))
    (:`then_1`
      (bind _output_get_3 (set `self.BlinkDelay` (+ _output_get (`self.BlinkDelay`)))))))

(event `EnhancedInput|/Game/LC/Input/IA_WS`
  (params (ActionValue :type "Float (double-precision)") (ElapsedSeconds :type "Float (double-precision)") (TriggeredSeconds :type "Float (double-precision)") (InputAction :type "InputAction Object Reference" :default "/Game/LC/Input/IA_WS.IA_WS"))
  (bind (_returnvalue_roll _returnvalue_pitch _returnvalue_yaw) (`KismetMathLibrary.BreakRotator` (`self.GetControlRotation`)))
  ; movement
  ;; ws movement
  (:`Triggered`
    (`self.AddMovementInput` (`KismetMathLibrary.GetForwardVector` (`KismetMathLibrary.MakeRotator` 0.0 0.0 _returnvalue_yaw)) ActionValue)))

(event `EnhancedInput|/Game/LC/Input/IA_Attack`
  (params (ActionValue :type Boolean) (ElapsedSeconds :type "Float (double-precision)") (TriggeredSeconds :type "Float (double-precision)") (InputAction :type "InputAction Object Reference" :default "/Game/LC/Input/IA_Attack.IA_Attack"))
  ; attack
  (:`Started`
    (if (>= (stale `self.ReceiveTick` _output_get_2) 2.0)
      (set `self.AttackDelay` 0.0))))

(event `EnhancedInput|/Game/LC/Input/IA_AD`
  (params (ActionValue :type "Float (double-precision)") (ElapsedSeconds :type "Float (double-precision)") (TriggeredSeconds :type "Float (double-precision)") (InputAction :type "InputAction Object Reference" :default "/Game/LC/Input/IA_AD.IA_AD"))
  (bind (_returnvalue_roll _returnvalue_pitch _returnvalue_yaw) (`KismetMathLibrary.BreakRotator` (`self.GetControlRotation`)))
  ; movement
  ;; ad movement
  (:`Triggered`
    (`self.AddMovementInput` (`KismetMathLibrary.GetRightVector` (`KismetMathLibrary.MakeRotator` _returnvalue_roll 0.0 _returnvalue_yaw)) ActionValue)))

(event `EnhancedInput|/Game/LC/Input/IA_Ability`
  (params (ActionValue :type Boolean) (ElapsedSeconds :type "Float (double-precision)") (TriggeredSeconds :type "Float (double-precision)") (InputAction :type "InputAction Object Reference" :default "/Game/LC/Input/IA_Ability.IA_Ability"))
  (bind _camera (`self.Camera`))
  (bind _indicator (`self.Indicator`))
  (bind _indicator_2 (`self.Indicator`))
  ; blink
  (:`Triggered`
    (`/Engine/EditorBlueprintResources/StandardMacros.IsValid` _indicator :!label _label_2
      (:`Is Valid`
        (bind _returnvalue (>= (stale `self.ReceiveTick` _output_get_3) 3.0))
        (if _returnvalue
          (bind (_returnvalue_2 _returnvalue2) (`self.RayCalc`))
          (bind _outhit (`KismetSystemLibrary.LineTraceSingle` :`Start` _returnvalue_2 :`End` _returnvalue2 :`TraceChannel` "TraceTypeQuery1" :`DrawDebugType` "ForDuration"))
          (bind (_bblockinghit _binitialoverlap _time _distance _location _impactpoint _normal _impactnormal _physmat _hitactor _hitcomponent _hitbonename _bonename _hititem _elementindex _faceindex _tracestart _traceend) (`GameplayStatics.BreakHitResult` _outhit))
          (if _bblockinghit
            (`self.K2_SetActorLocation` _indicator _location false false)
            (else
              (`self.K2_SetActorLocation` _indicator _traceend false false)))))
      (:`Is Not Valid`
        (if _returnvalue
          (bind (_returnvalue_3 _returnvalue2_2) (`self.RayCalc`))
          (bind _outhit_2 (`KismetSystemLibrary.LineTraceSingle` :`Start` _returnvalue_3 :`End` _returnvalue2_2 :`TraceChannel` "TraceTypeQuery1" :`DrawDebugType` "ForDuration"))
          (bind (_bblockinghit_2 _binitialoverlap_2 _time_2 _distance_2 _location_2 _impactpoint_2 _normal_2 _impactnormal_2 _physmat_2 _hitactor_2 _hitcomponent_2 _hitbonename_2 _bonename_2 _hititem_2 _elementindex_2 _faceindex_2 _tracestart_2 _traceend_2) (`GameplayStatics.BreakHitResult` _outhit_2))
          (if _bblockinghit_2
            (bind _returnvalue_4 (`|SpawnActorFromClass` "/Game/LC/Blueprint/BP_BlinkIndicator.BP_BlinkIndicator_C" (`KismetMathLibrary.MakeTransform` _location_2) "Undefined" "MultiplyWithRoot" null null))
            (set `self.Indicator` _returnvalue_4)
            (else
              (bind _returnvalue_5 (`|SpawnActorFromClass` "/Game/LC/Blueprint/BP_BlinkIndicator.BP_BlinkIndicator_C" (`KismetMathLibrary.MakeTransform` _traceend_2) "Undefined" "MultiplyWithRoot" null null))
              (set `self.Indicator` _returnvalue_5)))))))
  (:`Started`
    (goto _label_2))
  (:`Completed`
    (`/Engine/EditorBlueprintResources/StandardMacros.IsValid` _indicator_2
      (:`Is Valid`
        (if _returnvalue
          (`self.K2_SetActorLocation` (`self.K2_GetActorLocation` _indicator_2))
          (`self.K2_DestroyActor` _indicator_2)
          (bind (_direction _newtrack_0) (`Timeline|blinkeffect` :!via `PlayFromStart`)
            (:`Update`
              (`CameraComponent.SetFieldOfView` _camera _newtrack_0)
              (set `CameraComponent.PostProcessSettings` (make `PostProcessSettings` :`VignetteIntensity` (`KismetMathLibrary.MapRangeClamped` _newtrack_0 90.0 150.0 0.0 1.0)) _camera)
              (set `self.BlinkDelay` 0.0))))))))

(event `EnhancedInput|/Game/LC/Input/IA_Sprint`
  (params (ActionValue :type Boolean) (ElapsedSeconds :type "Float (double-precision)") (TriggeredSeconds :type "Float (double-precision)") (InputAction :type "InputAction Object Reference" :default "/Game/LC/Input/IA_Sprint.IA_Sprint"))
  ; sprint
  (:`Started`
    (set `CharacterMovementComponent.MaxWalkSpeed` 1200.0 (`self.CharacterMovement`)))
  (:`Completed`
    (set `CharacterMovementComponent.MaxWalkSpeed` 600.0 (`self.CharacterMovement`))))

(event `Key|F`
  (params (Key :type "Key Structure"))
  (bind _returnvalue (`self.K2_GetActorLocation`))
  (bind _ref_pose (`self.REF Pose`))
  (bind _returnvalue_2 (`SceneComponent.K2_GetComponentLocation` _ref_pose))
  (bind _returnvalue_3 (`SceneComponent.K2_GetComponentRotation` _ref_pose))
  ;[0.1356 0.07421 0.15 0.502] 암살 로직
  (:`Pressed`
    (bind (_outactors _returnvalue_4) (`KismetSystemLibrary.SphereOverlapActors` _returnvalue 200.0 (`|MakeArray` "ObjectTypeQuery10" "ObjectTypeQuery7" :!type "EObjectTypeQuery Enum")))
    (`KismetSystemLibrary.DrawDebugSphere` _returnvalue 200.0 12 (struct :`R` 0.061687 :`G` 1.0 :`A` 1.0) 5.0)
    (if _returnvalue_4
      (for _array_element _outactors
        (if (`self.ActorHasTag` _array_element "NPC")
          (bind _asbp_runawaynpc (cast `/Game/SHJ/BP/BP_RUNAWAYNPC` _array_element))
          (if (not (`/Game/SHJ/BP/BP_RUNAWAYNPC.IsDead` _asbp_runawaynpc))
            (`/Game/SHJ/BP/BP_RUNAWAYNPC.Move To` _asbp_runawaynpc _returnvalue_2 _returnvalue_3)
            (set `/Game/SHJ/BP/BP_RUNAWAYNPC.IsDead` true _asbp_runawaynpc)
            (`self.DisableInput` null :!label _label_3)
            (`self.PlayAnimMontage` "/Game/SHJ/Animation/Paired_Knife_Stealth_KidneyAndNeck_Att_Montage.Paired_Knife_Stealth_KidneyAndNeck_Att_Montage")
            (`KismetSystemLibrary.Delay` 2.0)
            (`self.EnableInput` null))
          (elif (`self.ActorHasTag` _array_element "Enemy")
            (bind _asbp_enemy (cast `/Game/NZW/01_Blueprints/BP_Enemy` _array_element))
            (if (not (`/Game/NZW/01_Blueprints/BP_Enemy.IsDead` _asbp_enemy))
              (`/Game/NZW/01_Blueprints/BP_Enemy.StealthDead` _asbp_enemy _returnvalue_2 _returnvalue_3)
              (goto _label_3))))))))

(fn `GetHit`)

(fn `Interaction Trace`
  (bind _camera (`self.Camera`))
  (bind _returnvalue (`SceneComponent.K2_GetComponentLocation` _camera))
  (bind _outhit (`KismetSystemLibrary.SphereTraceSingle` _returnvalue (+ _returnvalue (* (`KismetMathLibrary.GetForwardVector` (`SceneComponent.K2_GetComponentRotation` _camera)) 1000.0)) 3.0 "TraceTypeQuery1"))
  (bind (_bblockinghit _binitialoverlap _time _distance _location _impactpoint _normal _impactnormal _physmat _hitactor) (`GameplayStatics.BreakHitResult` _outhit))
  (if (`KismetSystemLibrary.DoesImplementInterface` _hitactor "/Game/SHJ/BP/BP_Interaction.BP_Interaction_C")
    (if (!= _hitactor (`self.Trace item`))
      (bind _output_get (set `self.Trace item` _hitactor))
      (message `/Game/SHJ/BP/BP_Interaction.Can Receive Trace` _output_get true))
    (else
      (message `/Game/SHJ/BP/BP_Interaction.Can Receive Trace` (`self.Trace item`) false)
      (set `self.Trace item` null))))

(fn `MappingContext`
  (bind _returnvalue (`GameplayStatics.GetPlayerController` 0))
  (`EnhancedInputSubsystemInterface.AddMappingContext` (pcsubsystem `EnhancedInputLocalPlayerSubsystem` (`GameplayStatics.GetPlayerController` 0)) "/Game/LC/Input/IMC_Player.IMC_Player" 0 (struct))
  (set `PlayerController.bShowMouseCursor` false _returnvalue)
  (`WidgetBlueprintLibrary.SetInputMode_GameOnly` _returnvalue))

(fn `MoveFunction`
  (params (A :type "Float (single-precision)"))
  (`self.K2_SetActorLocation` (+ (* (`self.movement_speed`) (`KismetMathLibrary.Normal` (+ (* (`|GetInputActionValue`) (0.0 0.0 0.0)) (* (`|GetInputActionValue`) (`self.GetActorForwardVector`)))) A) (`self.K2_GetActorLocation`))))

(fn `RayCalc`
  (returns (ReturnValue :type "Vector Structure") (ReturnValue2 :type "Vector Structure"))
  (bind _camera (`self.Camera`))
  (bind _returnvalue (`SceneComponent.K2_GetComponentLocation` _camera))
  (return _returnvalue (+ _returnvalue (* (`SceneComponent.GetForwardVector` _camera) 1000.0))))

(fn `UserConstructionScript`)